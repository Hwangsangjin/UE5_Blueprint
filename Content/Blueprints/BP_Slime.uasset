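; BP_Slime is a slime actor that moves along the world X axis at an erratic speed, as if racing toward a finish.
; Each Tick adds a random, delta-time-scaled step in positive X without sweeping, then clamps the position at a fixed X limit.
; Any actor overlap sets an Arrived flag, which this Blueprint never reads and which does not stop the movement.
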(event `self.ReceiveActorBeginOverlap`
  (params (OtherActor :type "Actor Object Reference"))
  (set `self.bArrived` true))

(event `self.ReceiveTick`
  (params (DeltaSeconds :type "Float (single-precision)"))
  (bind _returnvalue_x (`KismetMathLibrary.BreakVector` (`self.K2_GetActorLocation`)))
  (bind (_returnvalue_x_2 _returnvalue_y _returnvalue_z) (`KismetMathLibrary.BreakVector` (`self.K2_GetActorLocation`)))
  (`self.K2_SetActorLocation` (+ (`self.K2_GetActorLocation`) (`KismetMathLibrary.MakeVector` (* DeltaSeconds (`KismetMathLibrary.RandomFloatInRange` 50.0 3000.0)))))
  (if (>= _returnvalue_x 3750.0)
    (`self.K2_SetActorLocation` (`KismetMathLibrary.MakeVector` 3750.0 _returnvalue_y _returnvalue_z))))

(fn `UserConstructionScript`)